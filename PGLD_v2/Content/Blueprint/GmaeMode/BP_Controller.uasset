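; BP_Controller switches streaming levels from the number keys and NumPad 0, and toggles Ultra Dynamic Sky's time of day with W.
; Each level key sets ViewCount and shows a fade widget before StartUnload runs.
; StartUnload re-calls itself through the M_LevelSelect macro to blocking-unload every level in LevelName.
; It then removes W_MainUI, streams in the chosen level, sets the view to the first CineCameraActor and removes the fade.
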(event `Key|Zero`
  (params (Key :type "Key Structure"))
  ;[1 1 1] LV
  (:`Pressed`
    (set `self.ViewCount` 0)
    (bind _returnvalue (`|CreateWidget` "/Game/WIP/TA_PJH/UI/MainLV/W_Fade_In_Out.W_Fade_In_Out_C" :!label _label))
    (`UserWidget.AddToViewport` _returnvalue 0)
    (`/Game/WIP/TA_PJH/UI/MainLV/W_Fade_In_Out.E_FadeOut` _returnvalue)
    (`KismetSystemLibrary.Delay` 0.2)
    (`self.Start Unload` 0)))

(event `Key|One`
  (params (Key :type "Key Structure"))
  ;[1 1 1] LV
  (:`Pressed`
    (set `self.ViewCount` 1)
    (goto _label)))

(event `Key|Two`
  (params (Key :type "Key Structure"))
  ;[1 1 1] LV
  (:`Pressed`
    (set `self.ViewCount` 2)
    (goto _label)))

(event `Key|Three`
  (params (Key :type "Key Structure"))
  ;[1 1 1] LV
  (:`Pressed`
    (set `self.ViewCount` 3)
    (goto _label)))

(event `Key|Four`
  (params (Key :type "Key Structure"))
  ;[1 1 1] LV
  (:`Pressed`
    (set `self.ViewCount` 4)
    (goto _label)))

(event `Start Unload`
  (params (Index :type Integer))
  (bind _level_name (`self.Level_Name`))
  (bind _output (`|GetArrayItem` _level_name (`self.ViewCount`)))
  ;[1 1 1] LV
  (bind _index (`self.M_LevelSelect` Index _level_name)
    (:`Return`
      (`self.Start Unload` _index))
    (:`Out`
      ;;[1 1 1] Remove
      (bind _foundwidgets (`WidgetBlueprintLibrary.GetAllWidgetsOfClass` "/Game/WIP/TA_PJH/UI/MainLV/W_MainUI.W_MainUI_C"))
      (for _array_element _foundwidgets
        (`Widget.RemoveFromParent` _array_element))
      (`GameplayStatics.LoadStreamLevel` _output)
      (set `LevelStreaming.bShouldBeVisible` true (`GameplayStatics.GetStreamingLevel` _output))
      (`KismetSystemLibrary.Delay` 1.0)
      (bind _outactors (`GameplayStatics.GetAllActorsOfClass` "/Script/CinematicCamera.CineCameraActor"))
      (`self.SetViewTargetWithBlend` (`GameplayStatics.GetPlayerController` 0) (`|GetArrayItem` _outactors) 0.0 "VTBlend_Linear" 0.0 false)
      (`Widget.RemoveFromParent` (stale `Key|Zero` _returnvalue)))))

(event `Key|Five`
  (params (Key :type "Key Structure"))
  ;[1 1 1] LV
  (:`Pressed`
    (set `self.ViewCount` 5)
    (goto _label)))

(event `Key|Six`
  (params (Key :type "Key Structure"))
  ;[1 1 1] LV
  (:`Pressed`
    (set `self.ViewCount` 6)
    (goto _label)))

(event `Key|Seven`
  (params (Key :type "Key Structure"))
  ;[1 1 1] LV
  (:`Pressed`
    (set `self.ViewCount` 7)
    (goto _label)))

(event `Key|Eight`
  (params (Key :type "Key Structure"))
  ;[1 1 1] LV
  (:`Pressed`
    (set `self.ViewCount` 8)
    (goto _label)))

(event `Key|Nine`
  (params (Key :type "Key Structure"))
  ;[1 1 1] LV
  (:`Pressed`
    (set `self.ViewCount` 9)
    (goto _label)))

(event `Key|NumPadZero`
  (params (Key :type "Key Structure"))
  ;[1 1 1] LV
  (:`Pressed`
    (set `self.ViewCount` 10)
    (goto _label)))

(event `Key|W`
  (params (Key :type "Key Structure"))
  (:`Pressed`
    (bind _outactors (`GameplayStatics.GetAllActorsOfClass` "/Game/UltraDynamicSky/Blueprints/Ultra_Dynamic_Sky.Ultra_Dynamic_Sky_C"))
    (if (>= (`self.LIghtCount`) 1)
      (bind _output (`|GetArrayItem` _outactors))
      (set `/Game/UltraDynamicSky/Blueprints/Ultra_Dynamic_Sky.Time of Day` 1850.0 _output)
      (set `self.LIghtCount` 0)
      (else
        (set `/Game/UltraDynamicSky/Blueprints/Ultra_Dynamic_Sky.Time of Day` 1000.0 _output)
        (`/Engine/EditorBlueprintResources/StandardMacros.IncrementInt` (`self.LIghtCount`))))))

(fn `UserConstructionScript`)