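; BP_PlayMovie plays the looping movie chosen by the KTXSelection index on its WKTX reference.
; The PlayMovie1 event uses that index to pick a source from PlayerList and the matching entries in MoviePlayer and MovieTexture.
; It rewinds and closes the player, binds it to the texture, enables looping, then after a short delay latently opens the source and plays it.
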(event `PlayMovie1`
  (bind _ktxselection (`/Game/WIP/TA_PJH/UI/KTX/W_KTX.KTXSelection` (`self.W_KTX`)))
  (bind _output (`|GetArrayItem` (`self.Movie_Player`) _ktxselection))
  (bind _returnvalue (`MediaPlaylist.Get` (`self.PlayerList`) _ktxselection))
  (`MediaPlayer.Rewind` _output)
  (`MediaPlayer.Close` _output)
  (`MediaTexture.SetMediaPlayer` (`|GetArrayItem` (`self.Movie_Texture`) _ktxselection) _output)
  (`MediaPlayer.SetLooping` _output true)
  (`KismetSystemLibrary.Delay` 0.2)
  (`MediaPlayer.OpenSourceLatent` _output _returnvalue (make `MediaPlayerOptions` (struct :`Caption` -1 :`Metadata` -1 :`Script` -1 :`Subtitle` -1 :`Text` -1) "+00000000.00:00:00.000000000" "Enabled" "Enabled"))
  (`MediaPlayer.Play` _output))

(fn `UserConstructionScript`)